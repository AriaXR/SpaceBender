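; FixedBorder is an actor Blueprint that draws a fixed square debug border and a debug plane.
; BeginPlay stores four corner vertices of the square, while Tick redraws the box and plane with hard-coded sizes and a lingering duration.
; A minimum-area rectangle calculation over those vertices is disconnected from execution, so the box rotation reads its unset output and the derived extent is unused.
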(event EventBeginPlay
  (Variables|Default|Setvertices (Utilities|Array|MakeArray "-200.000000,-200.000000,0.000000" "-200.000000,200.000000,0.000000" "200.000000,200.000000,0.000000" "200.000000,-200.000000, 0")))

(event Collision|EventActorBeginOverlap
  (params (OtherActor :type Actor%20Object%20Reference)))

(event EventTick
  (params (DeltaSeconds :type Float%20%28single-precision%29))
  (Rendering|Debug|DrawDebugBox "0, 0, 0" "200.000000,200.000000, 0" "(R=0.128472,G=0.489622,B=0.770833,A=1.000000)" (stale _outrectrotation) 5.0 5e+01)
  (Class|KismetSystemLibrary|DrawDebugPlane (Utilities|Struct|MakePlane 1.0 0.0 0.0 0.0) "0, 0, 0" 2e+02 "(R=1.000000,G=1.000000,B=1.000000,A=1.000000)" 5.0))

(fn ConstructionScript)